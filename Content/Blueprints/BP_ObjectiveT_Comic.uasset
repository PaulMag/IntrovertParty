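; BP_ObjectiveT_Comic is an objective actor where the player, TheIntrovert, returns a comic.
; Tick polls for overlap with the player, enabling interaction on the character and setting the game mode's objective type to the comic's ID.
; When the player's just-interacted flag is set during overlap, it marks the comic returned on the game mode, clears the flag and destroys itself.
; The collision box's end-overlap event disables interaction.
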(event OnComponentEndOverlap(CollisionBox)
  (params (OverlappedComponent :type Primitive%20Component%20Object%20Reference) (OtherActor :type Actor%20Object%20Reference) (OtherComp :type Primitive%20Component%20Object%20Reference) (OtherBodyIndex :type Integer))
  (bind _asthe_introvert (Utilities|Casting|CastToTheIntrovert (Game|GetPlayerCharacter 0)))
  (Variables|/Script/IntrovertAtParty.TheIntrovert|SetobjectiveCanInteract _asthe_introvert false))

(event EventBeginPlay)

(event EventTick
  (params (DeltaSeconds :type Float%20%28single-precision%29))
  (bind _asthe_introvert (Utilities|Casting|CastToTheIntrovert (Game|GetPlayerCharacter 0)))
  (if (Collision|IsOverlappingActor _asthe_introvert :!class /Script/Engine.Actor)
    (Variables|/Script/IntrovertAtParty.TheIntrovert|SetobjectiveCanInteract _asthe_introvert true)
    (bind _asintrovert_at_party_game_mode_base (Utilities|Casting|CastToIntrovertAtPartyGameModeBase (Game|GetGameMode)))
    (Variables|/Script/IntrovertAtParty.IntrovertAtPartyGameModeBase|SetobjectiveType _asintrovert_at_party_game_mode_base 3)
    (bind _asthe_introvert_2 (Utilities|Casting|CastToTheIntrovert (Game|GetPlayerCharacter 0)))
    (if (Variables|/Script/IntrovertAtParty.TheIntrovert|GetdidJustInteract _asthe_introvert_2)
      (Variables|/Script/IntrovertAtParty.IntrovertAtPartyGameModeBase|SethasReturnedComic _asintrovert_at_party_game_mode_base true)
      (Variables|/Script/IntrovertAtParty.TheIntrovert|SetdidJustInteract _asthe_introvert_2 false)
      (Actor|DestroyActor))))

(event Collision|EventActorBeginOverlap
  (params (OtherActor :type Actor%20Object%20Reference)))

(fn ConstructionScript)