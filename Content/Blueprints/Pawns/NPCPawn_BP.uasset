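; NPC pawn that switches between four directional idle and walk visuals relative to the player's TheIntrovert pawn.
; Each tick, the dot product of both forward vectors selects the FFB or BFB set, and velocity selects walk or idle.
; Only the matching component stays visible; the other three are hidden.
; A billboard rotation step and a sound call are present but never run.
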(event EventBeginPlay)

(event Collision|EventActorBeginOverlap
  (params (OtherActor :type Actor%20Object%20Reference)))

(event EventTick
  (params (DeltaSeconds :type Float%20%28single-precision%29))
  (bind _returnvalue (Transformation|GetVelocity))
  (bind _walk_b_fb (Variables|Default|GetWalk_B_FB))
  (bind _idle_f_fb (Variables|Default|GetIdle_F_FB))
  (bind _idle_b_fb (Variables|Default|GetIdle_B_FB))
  (bind _returnvalue_2 (Math|Vector|VectorLength _returnvalue))
  (bind _returnvalue_3 (> _returnvalue_2 0.1))
  (bind _asthe_introvert (Utilities|Casting|CastToTheIntrovert (Game|Player|GetPlayerPawn 0)))
  (if (and (< (Math|Vector|DotProduct (Math|Vector|Normalize (Transformation|GetActorForwardVector)) (Math|Vector|Normalize (Transformation|GetActorForwardVector _asthe_introvert))) 0.0) (> (Math|Vector|DotProduct (Math|Vector|Normalize (Transformation|GetActorForwardVector)) (Math|Vector|Normalize (Transformation|GetActorForwardVector _asthe_introvert))) -1.0))
    (if _returnvalue_3
      (Rendering|SetVisibility (Variables|Default|GetWalk_F_FB) true false)
      (Rendering|SetVisibility _idle_f_fb false false)
      (else
        (Rendering|SetVisibility _idle_f_fb true false)
        (Rendering|SetVisibility _idle_b_fb false false)))
    (elif _returnvalue_3
      (Rendering|SetVisibility _walk_b_fb true false)
      (Rendering|SetVisibility _idle_b_fb false false)
      (else
        (Rendering|SetVisibility _idle_b_fb true false)
        (Rendering|SetVisibility _walk_b_fb false false)))))

(fn ConstructionScript)