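; BP_TheIntrovert is an actor Blueprint, apparently the player's introvert character, that sets up the HUD and tracks a stress level.
; BeginPlay creates a PlayerHUD widget for the first player, stores it and adds it to the viewport, while the I key lowers StressLevel by a fixed step.
; Tick prints the display name of a self-typed reference whose cast is disconnected, as is the Awkwardness reset.
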(event EventBeginPlay
  (bind _returnvalue (UserInterface|CreateWidget "/Game/HUD/PlayerHUD.PlayerHUD_C" (Game|GetPlayerController 0)))
  (bind _output_get (Variables|Default|SetHUD%20Ref. _returnvalue))
  (UserInterface|Viewport|AddtoViewport _output_get 0))

(event Collision|EventActorBeginOverlap
  (params (OtherActor :type Actor%20Object%20Reference)))

(event EventTick
  (params (DeltaSeconds :type Float%20%28single-precision%29))
  (Development|PrintString (Utilities|GetDisplayName (stale _asbp_the_introvert))))

(event Input|KeyboardEvents|I
  (params (Key :type Key%20Structure))
  (:Pressed
    (Variables|Default|SetStress%20Level (- (Variables|Default|GetStress%20Level) 0.25))))

(fn ConstructionScript)